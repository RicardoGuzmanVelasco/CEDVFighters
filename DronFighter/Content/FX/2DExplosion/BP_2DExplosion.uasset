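; BP_2DExplosion is a short-lived effect actor that shows an animated 2D explosion on a plane with sound.
; BeginPlay starts the audio, applies a dynamic instance of Mat_2DExplosion to the plane, and sets a sub-second lifespan.
; An empty looping timer function serves only as a clock.
; Tick feeds that timer's elapsed time into the material's PhaseControl parameter to drive the animation.
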(event EventBeginPlay
  (Audio|Components|Audio|Play (Variables|Default|GetAudio) 0.0)
  (bind _returnvalue (Rendering|Material|CreateDynamicMaterialInstance "/Game/FX/2DExplosion/Mat_2DExplosion.Mat_2DExplosion" :!class /Script/Engine.KismetMaterialLibrary))
  (bind _output_get (Variables|Default|SetDynMat _returnvalue))
  (Rendering|Material|SetMaterial (Variables|Default|GetPlane) 0 _output_get)
  (Utilities|Time|SetTimerbyFunctionName 0 "AnimationTimer" 1.0 true)
  (Actor|SetLifeSpan 0.8))

(event EventTick
  (params (DeltaSeconds :type Float%20%28single-precision%29))
  (Rendering|Material|SetScalarParameterValue (Variables|Default|GetDynMat) "PhaseControl" (Class|KismetSystemLibrary|GetTimerElapsedTime 0 "AnimationTimer") :!class /Script/Engine.MaterialInstanceDynamic))

(fn ConstructionScript)

(fn AnimationTimer)