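; Boss cannon pawn with a configurable mesh that turns its yaw toward the player ship and fires projectiles.
; A looping timer with a period randomized at BeginPlay calls Shot, which spawns a projectile and plays a sound once CanShot is set.
; The Animate event ramps a dynamic glow material on the last mesh slot via timeline, then enables firing and continuous tracking.
; Tick also refreshes the health bar widget.
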(event Custom|OnShot
  ;[1 1 1] Custom event to pass parameter to timered funcion
  (if (Variables|Default|GetCanShot)
    (CallFunction|Shot (Math|Vector|GetForwardVector (Variables|Default|GetRoot)))))

(event Custom|Animate
  ;[1 1 1] Custom event to trigger glow animation, and after that they can shot
  (bind _glowcannon (Timeline|Timeline_0 Play)
    (:Update
      (Rendering|Material|SetScalarParameterValue (Variables|Default|GetGlowMat) "Glow" _glowcannon :!class /Script/Engine.MaterialInstanceDynamic))
    (:Finished
      (Variables|Default|SetCanShot true))))

(event EventBeginPlay
  ;[1 1 1] Begin Play Event
  (Utilities|Time|SetTimerbyFunctionName 0 "OnShot" (Math|Random|RandomFloatinRange 0.2 1.0) true)
  (bind _returnvalue (Rendering|Material|CreateDynamicMaterialInstance "/Game/MATERIALS/BossGlowCannon_Mat.BossGlowCannon_Mat" :!class /Script/Engine.KismetMaterialLibrary))
  (bind _output_get (Variables|Default|SetGlowMat _returnvalue))
  (CallFunction|SetGlowMaterial (Variables|Default|GetCannon) _output_get)
  (bind _ascannon_health_bar (Utilities|Casting|CastToCannonHealthBar (UserInterface|GetUserWidgetObject (Variables|Default|GetHealthBar))))
  (Class|ProgressBar|SetFillColorandOpacity (Variables|/Game/UI/Widgets/CannonHealthBar.CannonHealthBar_C|GetHealthBar _ascannon_health_bar) (Variables|Default|GetHealthBarColor))
  (CallFunction|LookatPlayer))

(event EventTick
  (params (DeltaSeconds :type Float%20%28single-precision%29))
  ;[1 1 1] Follows player ship movements
  (CallFunction|UpdateHealth)
  (if (Variables|Default|GetCanShot)
    (CallFunction|LookatPlayer)))

(fn ConstructionScript
  ;[1 1 1] To allow any mesh
  (Components|StaticMesh|SetStaticMesh (Variables|Default|GetCannon) (Variables|Default|GetCannonMesh)))

(fn Shot
  (params (Direction :type Vector))
  (bind _projoffset (Variables|Default|GetProjOffset))
  (bind _returnvalue (Transformation|GetWorldLocation _projoffset))
  (if (> (Math|Vector|VectorLength Direction) 0.0)
    ;[1 1 1] Spawn Projectile at location
    (Game|SpawnActorfromClass "/Game/PAWNS/BP_PlayerProj_Normal.BP_PlayerProj_Normal_C" (Math|Transform|MakeTransform _returnvalue (Math|Conversions|RotationFromXVector Direction)) "AlwaysSpawn" 0 0)
    ;[1 1 1] Play fire sound
    (Audio|PlaySoundatLocation (Variables|Default|GetFireSound) _returnvalue "0, 0, 0" 0.6)))

(fn SetGlowMaterial
  (params (Mesh :type Static%20Mesh%20Component%20Object%20Reference) (Material :type Material%20Instance%20Dynamic%20Object%20Reference))
  (Rendering|Material|SetMaterial Mesh (- (Utilities|Array|Length (Rendering|Material|GetMaterials Mesh)) 1) Material))

(fn UpdateHealth
  (bind _ascannon_health_bar (Utilities|Casting|CastToCannonHealthBar (UserInterface|GetUserWidgetObject (Variables|Default|GetHealthBar))))
  (Progress|SetPercent (Variables|/Game/UI/Widgets/CannonHealthBar.CannonHealthBar_C|GetHealthBar _ascannon_health_bar) (/ (Variables|Default|GetHealth) (Variables|Default|GetMaxHealth))))

(fn LookatPlayer
  (bind _root (Variables|Default|GetRoot))
  (bind _relativerotation (Variables|/Script/Engine.SceneComponent|GetRelativeRotation _root))
  (Transformation|SetRelativeRotation _root (Math|Rotator|MakeRotator (.roll _relativerotation) (.pitch _relativerotation) (.yaw (Math|Rotator|FindLookatRotation (Transformation|GetWorldLocation (Variables|Default|GetRoot)) (Transformation|GetActorLocation (Game|Player|GetPlayerPawn 0))))) false true))