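; Boss pawn for a multi-phase fight, driven by the game mode's GamePhase.
; Tick moves it to the BossFinalPosition target point to start combat, then expands it once four cannons are killed.
; Expansion chains timelines that slide platforms, covers and tower into place, then animates the long cannons.
; Destroying the tower cannon triggers Explode, which staggers randomized explosions through a delayed-loop macro, destroys the boss and opens TransitionLevel.
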(event Custom|OnExpand
  (bind _rightcover (Variables|Default|GetRightCover))
  (bind _leftcover (Variables|Default|GetLeftCover))
  (bind _rightplatform (Variables|Default|GetRightPlatform))
  (bind _leftplatform (Variables|Default|GetLeftPlatform))
  (bind _towercannon (Variables|Default|GetTowerCannon))
  (bind _rightplatform_2 (Variables|Default|GetRightPlatform))
  (bind _leftplatform_2 (Variables|Default|GetLeftPlatform))
  (bind _leftcover_2 (Variables|Default|GetLeftCover))
  (bind _rightcover_2 (Variables|Default|GetRightCover))
  (bind _relativelocation (Variables|/Script/Engine.SceneComponent|GetRelativeLocation _rightcover))
  (bind _relativelocation_2 (Variables|/Script/Engine.SceneComponent|GetRelativeLocation _leftcover))
  (bind _relativelocation_3 (Variables|/Script/Engine.SceneComponent|GetRelativeLocation _rightplatform))
  (bind _relativelocation_4 (Variables|/Script/Engine.SceneComponent|GetRelativeLocation _leftplatform))
  (bind _relativelocation_5 (Variables|/Script/Engine.SceneComponent|GetRelativeLocation _rightplatform_2))
  (bind _relativelocation_6 (Variables|/Script/Engine.SceneComponent|GetRelativeLocation _leftplatform_2))
  (bind _relativelocation_7 (Variables|/Script/Engine.SceneComponent|GetRelativeLocation _rightcover_2))
  (bind _relativelocation_8 (Variables|/Script/Engine.SceneComponent|GetRelativeLocation _leftcover_2))
  (bind _relativelocation_9 (Variables|/Script/Engine.SceneComponent|GetRelativeLocation _towercannon))
  ;[0.4471 0.1373 1] Phase Condition
  (if (Utilities|Enum|Equal(Enum) (Variables|/Script/CEDVFighters.CEDVFightersGameMode|GetGamePhase (Variables|Default|GetGameModeRef)) "GPHASE_BossCombat")
    ;[0.4471 0.1373 1] Set Phase
    (Variables|/Script/CEDVFighters.CEDVFightersGameMode|SetGamePhase (Variables|Default|GetGameModeRef) "GPHASE_BossExpanding")
    ;[0.3245 0.7009 1] Boss animation
    (Audio|PlaySound2D "/Game/SOUND/GAME/Transformer.Transformer")
    (bind _h_offsetplatform (Timeline|TimeLine_PlatformH Play)
      (:Update
        (Transformation|SetRelativeLocation _rightplatform_2 (Math|Vector|MakeVector _h_offsetplatform (.y _relativelocation_5) (.z _relativelocation_5)) false true)
        (Transformation|SetRelativeLocation _leftplatform_2 (Math|Vector|MakeVector (* _h_offsetplatform -1.0) (.y _relativelocation_6) (.z _relativelocation_6)) false true))
      (:Finished
        (bind _v_offsetplatform (Timeline|TimeLine_PlatformV Play)
          (:Update
            (Transformation|SetRelativeLocation _rightplatform (Math|Vector|MakeVector (.x _relativelocation_3) (.y _relativelocation_3) _v_offsetplatform) false true)
            (Transformation|SetRelativeLocation _leftplatform (Math|Vector|MakeVector (.x _relativelocation_4) (.y _relativelocation_4) _v_offsetplatform) false true))
          (:Finished
            (bind _v_offsetcover (Timeline|Timeline_CoverV Play)
              (:Update
                (Transformation|SetRelativeLocation _rightcover_2 (Math|Vector|MakeVector (.x _relativelocation_7) (.y _relativelocation_7) _v_offsetcover) false true)
                (Transformation|SetRelativeLocation _leftcover_2 (Math|Vector|MakeVector (.x _relativelocation_8) (.y _relativelocation_8) _v_offsetcover) false true))
              (:Finished
                (bind _h_offsetcover (Timeline|Timeline_CoverH Play)
                  (:Update
                    (Transformation|SetRelativeLocation _rightcover (Math|Vector|MakeVector _h_offsetcover (.y _relativelocation) (.z _relativelocation)) false true)
                    (Transformation|SetRelativeLocation _leftcover (Math|Vector|MakeVector (* _h_offsetcover -1.0) (.y _relativelocation_2) (.z _relativelocation_2)) false true))
                  (:Finished
                    (bind _v_offsettwer (Timeline|Timeline_TowerV Play)
                      (:Update
                        (Transformation|SetRelativeLocation _towercannon (Math|Vector|MakeVector (.x _relativelocation_9) (.y _relativelocation_9) _v_offsettwer) false true))
                      (:Finished
                        (bind _asbp_long_cannon (Utilities|Casting|CastToBP_LongCannon (Variables|/Script/Engine.ChildActorComponent|GetChildActor (Variables|Default|GetRightPlatformCannon))))
                        (Default|Animate _asbp_long_cannon)
                        (bind _asbp_long_cannon_2 (Utilities|Casting|CastToBP_LongCannon (Variables|/Script/Engine.ChildActorComponent|GetChildActor (Variables|Default|GetLeftPlatformCannon))))
                        (Default|Animate _asbp_long_cannon_2)
                        (bind _asbp_long_cannon_3 (Utilities|Casting|CastToBP_LongCannon (Variables|/Script/Engine.ChildActorComponent|GetChildActor (Variables|Default|GetTowerCannon))))
                        (Default|Animate _asbp_long_cannon_3)
                        ;[0.4471 0.1373 1] Set Phase
                        (Variables|/Script/CEDVFighters.CEDVFightersGameMode|SetGamePhase (Variables|Default|GetGameModeRef) "GPHASE_BossExpanded")))))))))))))

(event Custom|Explode
  (bind _returnvalue (Transformation|GetActorTransform))
  (bind _returnvalue_2 (Math|Random|RandomFloatinRange 0.6 2.0))
  (bind _tp_finalposition (Variables|Default|GetTP_FinalPosition))
  (bind _returnvalue_3 (Transformation|GetActorLocation _tp_finalposition))
  ;[1 1 1] Boss explosion
  (Rendering|SetVisibility (Variables|Default|GetDefaultSceneRoot) false true)
  (Game|SpawnActorfromClass "/Game/PAWNS/BP_BossExplosion.BP_BossExplosion_C" (Math|Transform|MakeTransform (Math|Vector|MakeVector (.x (.location _returnvalue)) (.y (.location _returnvalue)) 2e+02) (.rotation _returnvalue) (.scale _returnvalue)) "Undefined" 0 0)
  (Utilities|FlowControl|Delay 0.8)
  (Utilities|LoopwithDelay 0 16 0.1
    (:Loop%20Body
      (bind _explosionclass (CallFunction|GetRandomExplosion))
      (Game|SpawnActorfromClass _explosionclass (Math|Transform|MakeTransform (Math|Vector|MakeVector (+ (Math|Random|RandomFloatinRange -5e+02 5e+02) (.x _returnvalue_3)) (+ (.y _returnvalue_3) (Math|Random|RandomFloatinRange -5e+02 5e+02)) 4e+02) "0, 0, 0" (Math|Vector|MakeVector _returnvalue_2 _returnvalue_2 1.0)) "Undefined" 0 0))
    (:Completed
      (Actor|DestroyActor)
      (Development|PrintString "HelloME CAGO EN LA PUTA")
      (Game|OpenLevel(byName) "TransitionLevel" false))))

(event EventBeginPlay
  ;[1 1 1] Get Game Mode reference and Target Point for boss final position
  (bind _ascedvfighters_game_mode (Utilities|Casting|CastToCEDVFightersGameMode (Game|GetGameMode)))
  (Variables|Default|SetGameModeRef _ascedvfighters_game_mode)
  (bind _outactors (Actor|GetAllActorsOfClass "/Script/Engine.TargetPoint"))
  (for _array_element _outactors
    (if (Utilities|Enum|Equal(Enum) (Utilities|GetDisplayName _array_element) "BossFinalPosition")
      (Variables|Default|SetTP_FinalPosition _array_element))))

(event EventTick
  (params (DeltaSeconds :type Float%20%28single-precision%29))
  (bind _towercannon (Variables|Default|GetTowerCannon))
  ;[1 1 1] Tick event
  ;;[1 1 1] Approach phase
  (CallFunction|ApproachMove DeltaSeconds)
  ;;[1 1 1] Boss in second combat phase?
  (if (Utilities|Enum|Equal(Enum) (Variables|/Script/CEDVFighters.CEDVFightersGameMode|GetGamePhase (Variables|Default|GetGameModeRef)) "GPHASE_BossExpanded")
    ;;[1 1 1] Kill Boss if we killed tower cannon
    (Utilities|IsValid _towercannon
      (:Is%20Valid
        (bind _asbp_long_cannon (Utilities|Casting|CastToBP_LongCannon (Variables|/Script/Engine.ChildActorComponent|GetChildActor _towercannon)))
        (Utilities|IsValid _asbp_long_cannon
          (:Is%20Valid
            (if (<= (Variables|/Game/PAWNS/BP_LongCannon.BP_LongCannon_C|GetHealth _asbp_long_cannon) 0.0)
              (CallFunction|Explode :!label _label)
              (Variables|/Script/CEDVFighters.CEDVFightersGameMode|SetGamePhase (Variables|Default|GetGameModeRef) "GPHASE_BossKilled")))
          (:Is%20Not%20Valid
            (goto _label)))))
    (else
      ;;[1 1 1] Expand Boss if we killed 4 cannons
      (if (== (Variables|/Script/CEDVFighters.CEDVFightersGameMode|GetKilledCannons (Variables|Default|GetGameModeRef)) 4)
        (CallFunction|OnExpand)))))

(fn ConstructionScript)

(fn SetGlowMaterial
  (params (Material :type Material%20Instance%20Dynamic%20Object%20Reference) (Mesh :type Static%20Mesh%20Component%20Object%20Reference))
  (Rendering|Material|SetMaterial Mesh (- (Utilities|Array|Length (Rendering|Material|GetMaterials Mesh)) 1) Material))

(fn ApproachMove
  (params (DeltaSeconds :type Float%20%28single-precision%29))
  (if (Utilities|Enum|Equal(Enum) (Variables|/Script/CEDVFighters.CEDVFightersGameMode|GetGamePhase (Variables|Default|GetGameModeRef)) "GPHASE_BossSpawn")
    (Class|MovementComponent|MoveUpdatedComponent (Variables|Default|GetProjectileMovement) (* (Variables|/Script/Engine.MovementComponent|GetVelocity (Variables|Default|GetProjectileMovement)) DeltaSeconds) (Transformation|GetActorRotation) true)
    (if (Math|Vector|Equal(Vector) (Transformation|GetActorLocation) (Transformation|GetActorLocation (Variables|Default|GetTP_FinalPosition)) 5e+01)
      (Variables|/Script/CEDVFighters.CEDVFightersGameMode|SetGamePhase (Variables|Default|GetGameModeRef) "GPHASE_BossCombat"))))

(fn GetRandomExplosion
  (bind _explosions (LocalVariables|GetExplosions))
  (return (Utilities|Array|Get(acopy) _explosions (Math|Random|RandomIntegerinRange 0 (- (Utilities|Array|Length _explosions) 1)))))