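; Boss actor that plays a staged mechanical unfolding sequence of its platforms, covers and tower cannon when OnExpand fires.
; Five chained timelines move the platforms sideways then vertically, the covers vertically then sideways, and finally the tower cannon vertically.
; Each timeline drives one relative axis with teleport moves, negating the horizontal offset to mirror left and right parts.
; BeginPlay, overlap and construction logic are empty.
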(event Custom|OnExpand
  (bind _rightcover (Variables|Default|GetRightCover))
  (bind _leftcover (Variables|Default|GetLeftCover))
  (bind _rightplatform (Variables|Default|GetRightPlatform))
  (bind _leftplatform (Variables|Default|GetLeftPlatform))
  (bind _towercannon (Variables|Default|GetTowerCannon))
  (bind _rightplatform_2 (Variables|Default|GetRightPlatform))
  (bind _leftplatform_2 (Variables|Default|GetLeftPlatform))
  (bind _leftcover_2 (Variables|Default|GetLeftCover))
  (bind _rightcover_2 (Variables|Default|GetRightCover))
  (bind _relativelocation (Variables|/Script/Engine.SceneComponent|GetRelativeLocation _rightcover))
  (bind _relativelocation_2 (Variables|/Script/Engine.SceneComponent|GetRelativeLocation _leftcover))
  (bind _relativelocation_3 (Variables|/Script/Engine.SceneComponent|GetRelativeLocation _rightplatform))
  (bind _relativelocation_4 (Variables|/Script/Engine.SceneComponent|GetRelativeLocation _leftplatform))
  (bind _relativelocation_5 (Variables|/Script/Engine.SceneComponent|GetRelativeLocation _rightplatform_2))
  (bind _relativelocation_6 (Variables|/Script/Engine.SceneComponent|GetRelativeLocation _leftplatform_2))
  (bind _relativelocation_7 (Variables|/Script/Engine.SceneComponent|GetRelativeLocation _rightcover_2))
  (bind _relativelocation_8 (Variables|/Script/Engine.SceneComponent|GetRelativeLocation _leftcover_2))
  (bind _relativelocation_9 (Variables|/Script/Engine.SceneComponent|GetRelativeLocation _towercannon))
  (bind _h_offsetplatform (Timeline|TimeLine_PlatformH Play)
    (:Update
      (Transformation|SetRelativeLocation _rightplatform_2 (Math|Vector|MakeVector (.x _relativelocation_5) _h_offsetplatform (.z _relativelocation_5)) false true)
      (Transformation|SetRelativeLocation _leftplatform_2 (Math|Vector|MakeVector (.x _relativelocation_6) (* _h_offsetplatform -1.0) (.z _relativelocation_6)) false true))
    (:Finished
      (bind _v_offsetplatform (Timeline|TimeLine_PlatformV Play)
        (:Update
          (Transformation|SetRelativeLocation _rightplatform (Math|Vector|MakeVector (.x _relativelocation_3) (.y _relativelocation_3) _v_offsetplatform) false true)
          (Transformation|SetRelativeLocation _leftplatform (Math|Vector|MakeVector (.x _relativelocation_4) (.y _relativelocation_4) _v_offsetplatform) false true))
        (:Finished
          (bind _v_offsetcover (Timeline|Timeline_CoverV Play)
            (:Update
              (Transformation|SetRelativeLocation _rightcover_2 (Math|Vector|MakeVector (.x _relativelocation_7) (.y _relativelocation_7) _v_offsetcover) false true)
              (Transformation|SetRelativeLocation _leftcover_2 (Math|Vector|MakeVector (.x _relativelocation_8) (.y _relativelocation_8) _v_offsetcover) false true))
            (:Finished
              (bind _h_offsetcover (Timeline|Timeline_CoverH Play)
                (:Update
                  (Transformation|SetRelativeLocation _rightcover (Math|Vector|MakeVector (.x _relativelocation) _h_offsetcover (.z _relativelocation)) false true)
                  (Transformation|SetRelativeLocation _leftcover (Math|Vector|MakeVector (.x _relativelocation_2) (* _h_offsetcover -1.0) (.z _relativelocation_2)) false true))
                (:Finished
                  (bind _v_offsettwer (Timeline|Timeline_TowerV Play)
                    (:Update
                      (Transformation|SetRelativeLocation _towercannon (Math|Vector|MakeVector (.x _relativelocation_9) (.y _relativelocation_9) _v_offsettwer) false true))))))))))))

(event EventBeginPlay)

(event Collision|EventActorBeginOverlap
  (params (OtherActor :type Actor%20Object%20Reference)))

(fn ConstructionScript)